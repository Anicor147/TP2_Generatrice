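; BP_Screwdriver is a screwdriver item that the first-person character can grab.
; Interact casts the player character to BP_FirstPersonCharacter and passes the screwdriver to its GrabItem function.
; It records its root's world location on BeginPlay, and ReturnPosition moves it back there, leaving rotation untouched.
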(event `self.ReceiveBeginPlay`
  (set `self.Initial Location` (`SceneComponent.K2_GetComponentLocation` (`self.DefaultSceneRoot`))))

(event `/Game/Tp2/BPI_Interaction.Interact`
  (params (HitComponent :type "PrimitiveComponent Object Reference"))
  (bind _asbp_first_person_character (cast `/Game/FirstPerson/Blueprints/BP_FirstPersonCharacter` (`GameplayStatics.GetPlayerCharacter` 0)))
  (`/Game/FirstPerson/Blueprints/BP_FirstPersonCharacter.Grab Item` _asbp_first_person_character self))

(event `/Game/Tp2/BPI_Detach.ReturnPosition`
  (bind _output_get (set `self.Initial Location` (`self.Initial Location`)))
  (`SceneComponent.K2_SetWorldLocation` (`self.DefaultSceneRoot`) _output_get false false))

(fn `UserConstructionScript`)