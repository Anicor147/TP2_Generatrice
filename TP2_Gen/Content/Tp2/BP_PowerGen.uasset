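; BP_PowerGen is an interactable power generator puzzle that opens a linked door once repaired.
; Interacting with Screw-tagged components while holding a screwdriver drops them as physics objects, and the fourth screw also releases the cover.
; With all screws out, using a held generator battery on the battery slot consumes it, brightens the point light, powers on the widget display and messages the door to open.
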(event `/Game/Tp2/BPI_Interaction.Interact`
  (params (HitComponent :type "PrimitiveComponent Object Reference"))
  (bind _cover (`self.Cover`))
  ;[1 1 1] Vis
  (if (`ActorComponent.ComponentHasTag` HitComponent "Screw")
    (bind _asbp_first_person_character (cast `/Game/FirstPerson/Blueprints/BP_FirstPersonCharacter` (`GameplayStatics.GetPlayerCharacter` 0)))
    (cast `/Game/Tp2/BP_Screwdriver` (`/Game/FirstPerson/Blueprints/BP_FirstPersonCharacter.ItemHeld` _asbp_first_person_character))
    (`|ExecutionSequence`
      (:`then_0`
        (`SceneComponent.K2_DetachFromComponent` HitComponent "KeepWorld" "KeepRelative" "KeepRelative" true)
        (`PrimitiveComponent.SetSimulatePhysics` HitComponent true)
        (`PrimitiveComponent.SetCollisionEnabled` HitComponent "PhysicsOnly"))
      (:`then_1`
        (bind _result (`/Engine/EditorBlueprintResources/StandardMacros.IncrementInt` (`self.ScrewCounter`))
          (:`  `
            (if (== _result 4)
              (`SceneComponent.K2_DetachFromComponent` _cover "KeepWorld" "KeepRelative" "KeepRelative" true)
              (`PrimitiveComponent.SetSimulatePhysics` _cover true))))))
    (else
      ;[1 1 1] Battery
      (if (and (== HitComponent (`self.Battery Slot`)) (== (`self.ScrewCounter`) 4))
        (bind _asbp_first_person_character_2 (cast `/Game/FirstPerson/Blueprints/BP_FirstPersonCharacter` (`GameplayStatics.GetPlayerCharacter` 0)))
        (cast `/Game/Tp2/BP_GenBattery` (`/Game/FirstPerson/Blueprints/BP_FirstPersonCharacter.ItemHeld` _asbp_first_person_character_2))
        (`|ExecutionSequence`
          (:`then_0`
            (`LightComponent.SetIntensity` (`self.PointLight`) 10000.0))
          (:`then_1`
            (`/Game/FirstPerson/Blueprints/BP_FirstPersonCharacter.Destroy Item` _asbp_first_person_character_2))
          (:`then_2`
            (bind _aswbp_gen_display (cast `/Game/Tp2/WBP_GenDisplay` (`WidgetComponent.GetWidget` (`self.GenDisplay`))))
            (`/Game/Tp2/WBP_GenDisplay.Power On` _aswbp_gen_display))
          (:`then_3`
            (message `/Game/Tp2/BPI_OpenDoor.Open Door` (`self.Door`))))))))

(fn `UserConstructionScript`)